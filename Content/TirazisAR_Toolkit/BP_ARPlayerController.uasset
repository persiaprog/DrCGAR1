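; Player controller that runs an image-tracking AR app from welcome screen through scan, model spawn, rescan and quit prompt.
; A ProgramState enum drives the flow, with Tick polling AR geometries for a tracked image.
; Once the scan widget's progress animation confirms detection, it spawns AR_Model offset from the image and shows menu and success widgets.
; The session status check is disconnected, so StartAR assumes success; Android Back and Menu keys control quitting and menu.
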(event Custom|StartProgramClicked
  ;[1 1 1] Begin Play / Create Welcome Widget and add to viewport
  (Variables|Flag|SetProgramState "NewEnumerator1")
  (CallFunction|StartAR))

(event Custom|StartAR
  ;[1 1 1] Start AR Session / Remove Welcome Widget and Add Fit to Scan Widget to Viewport
  (Class|ARBlueprintLibrary|StartARSession "/Game/ProjectData/AR_Data/AR_SessionConfig.AR_SessionConfig")
  (Variables|Flag|SetProgramState "NewEnumerator2")
  (bind _welcomewidget (Variables|UI|GetWelcomeWidget)
    (:then
      (Widget|RemovefromParent _welcomewidget))
    (:else
      _))
  (bind _returnvalue (UserInterface|CreateWidget "/Game/TirazisAR_Toolkit/UI/WBP_FitToScanWidget.WBP_FitToScanWidget_C"))
  (bind _output_get (Variables|UI|SetFitToScanWidget _returnvalue))
  (EventDispatchers|BindEventtoProgressFinishedDisp _output_get (delegate Custom|ProgressFinished))
  (UserInterface|Viewport|AddtoViewport (Variables|UI|GetFitToScanWidget) 0)
  (CallFunction|StartImageTracking))

(event Custom|StopAR
  (Class|ARBlueprintLibrary|StopARSession))

(event Custom|MoveARModelZ
  (bind _armodel (Variables|Default|GetARModel))
  (bind _returnvalue (Transformation|GetActorLocation _armodel))
  (Transformation|SetActorLocation _armodel (Math|Vector|MakeVector (.x _returnvalue) (.y _returnvalue) (+ (.z _returnvalue) 5e+01)) true false))

(event Custom|MoveARModelX
  (bind _armodel (Variables|Default|GetARModel))
  (bind _returnvalue (Transformation|GetActorLocation _armodel))
  (Transformation|SetActorLocation _armodel (Math|Vector|MakeVector (+ (.x _returnvalue) 5e+01) (.y _returnvalue) (.z _returnvalue)) true false))

(event Custom|MoveARModelY
  (bind _armodel (Variables|Default|GetARModel))
  (bind _returnvalue (Transformation|GetActorLocation _armodel))
  (Transformation|SetActorLocation _armodel (Math|Vector|MakeVector (.x _returnvalue) (+ (.y _returnvalue) 5e+01) (.z _returnvalue)) true false))

(event Custom|ProgressFinished
  ;[1 1 1] Start AR Session / Remove Welcome Widget and Add Fit to Scan Widget to Viewport
  (Variables|Flag|SetImageTrackingAccurateProgressFinished true))

(event Custom|StartImageTracking
  ;[1 1 1] Enable Image Tracking Flag and Set Program State to AR Image Tracking
  (Variables|Flag|SetImageTrackingIsActivate true)
  (Variables|Flag|SetProgramState "NewEnumerator4"))

(event Custom|SpawnModel
  (bind _tracked_geometry (Variables|Default|GetTracked%20Geometry))
  (bind _returnvalue (Class|ARTrackedGeometry|GetLocaltoWorldTransform _tracked_geometry))
  (Utilities|IsValid (Variables|Default|GetARModel)
    (:Is%20Valid
      (Actor|DestroyActor (Variables|Default|GetARModel)))
    (:Is%20Not%20Valid
      _))
  (Variables|Flag|SetProgramState "NewEnumerator7")
  (bind _returnvalue_2 (Game|SpawnActorfromClass "/Game/ProjectData/AR_Model.AR_Model_C" (Math|Transform|MakeTransform (Math|Vector|MakeVector (- (.x (.location _returnvalue)) (Variables|Default|GetDistanceX)) (- (.y (.location _returnvalue)) (Variables|Default|GetDistanceY)) (- (.z (.location _returnvalue)) (Variables|Default|GetDistanceZ))) "0, 0, 0" "7.500000,7.500000,7.500000") "Undefined" 0 0))
  (Variables|Default|SetARModel _returnvalue_2)
  (bind _mainmenuwidget (Variables|UI|GetMainMenuWidget)
    (:then
      (Widget|RemovefromParent _mainmenuwidget))
    (:else
      _))
  (bind _returnvalue_3 (UserInterface|CreateWidget "/Game/TirazisAR_Toolkit/UI/WBP_MainMenuWidget.WBP_MainMenuWidget_C"))
  (bind _output_get (Variables|UI|SetMainMenuWidget _returnvalue_3))
  (UserInterface|Viewport|AddtoViewport _output_get 0)
  (bind _detectsuccesswidget (Variables|UI|GetDetectSuccessWidget)
    (:then
      (Widget|RemovefromParent _detectsuccesswidget))
    (:else
      _))
  (bind _returnvalue_4 (UserInterface|CreateWidget "/Game/TirazisAR_Toolkit/UI/WBP_DetectSuccessfulWidget.WBP_DetectSuccessfulWidget_C"))
  (bind _output_get_2 (Variables|UI|SetDetectSuccessWidget _returnvalue_4))
  (UserInterface|Viewport|AddtoViewport _output_get_2 0))

(event Custom|ShowQuitPrompt
  ;[1 1 1] Show Quit Prompt
  (bind _returnvalue (UserInterface|CreateWidget "/Game/TirazisAR_Toolkit/UI/WBP_QuitPrompt.WBP_QuitPrompt_C"))
  (EventDispatchers|BindEventtoDispNoButtonPressed _returnvalue (delegate Custom|QuitPrompt_NoButtonPressed))
  (UserInterface|Viewport|AddtoViewport _returnvalue 0)
  (Variables|Flag|SetQuitPromptIsShown? true))

(event Custom|QuitPrompt_NoButtonPressed
  ;[1 1 1] Show Quit Prompt
  (Variables|Flag|SetQuitPromptIsShown? false))

(event Custom|RestartARScan
  (bind _mainmenuwidget (Variables|UI|GetMainMenuWidget)
    (:then
      (Widget|RemovefromParent _mainmenuwidget))
    (:else
      _))
  (bind _armodel (Variables|Default|GetARModel)
    (:then
      (Actor|DestroyActor _armodel))
    (:else
      _))
  (CallFunction|StartAR))

(event Custom|ShowAboutWidget
  (Game|SetGamePaused true)
  (bind _returnvalue (UserInterface|CreateWidget "/Game/TirazisAR_Toolkit/UI/WBP_AboutWidget.WBP_AboutWidget_C"))
  (UserInterface|Viewport|AddtoViewport _returnvalue 0))

(event EventBeginPlay
  ;[1 1 1] Begin Play / Create Welcome Widget and add to viewport
  (bind _returnvalue (UserInterface|CreateWidget "/Game/TirazisAR_Toolkit/UI/WBP_WelcomePageWidget.WBP_WelcomePageWidget_C"))
  (bind _output_get (Variables|UI|SetWelcomeWidget _returnvalue))
  (EventDispatchers|BindEventtoStartProgramClickedDisp _output_get (delegate Custom|StartProgramClicked))
  (UserInterface|Viewport|AddtoViewport (Variables|UI|GetWelcomeWidget) 0))

(event EventTick
  (params (DeltaSeconds :type Float%20%28single-precision%29))
  (bind _fittoscanwidget (Variables|UI|GetFitToScanWidget))
  (bind _fittoscanwidget_2 (Variables|UI|GetFitToScanWidget))
  (if (Variables|Flag|GetImageTrackingIsActivate)
    (bind _trackedgeometry (CallFunction|ScanandDetectARImage))
    (Utilities|IsValid _trackedgeometry
      (:Is%20Valid
        (switch Utilities|FlowControl|Switch|SwitchonE_ProgramState (Variables|Flag|GetProgramState)
          (:NewEnumerator4
            (Variables|Flag|SetProgramState "NewEnumerator5")
            (Default|StartProgressBarAnimation _fittoscanwidget)
            (Default|ShowProgressCanvas _fittoscanwidget))
          (:NewEnumerator5
            (if (Variables|Flag|GetImageTrackingAccurateProgressFinished)
              (Variables|Flag|SetProgramState "NewEnumerator6")
              (Variables|Default|SetTracked%20Geometry _trackedgeometry)
              (Variables|Flag|SetImageTrackingIsActivate false)
              (Variables|Flag|SetImageTrackingAccurateProgressFinished false)))))
      (:Is%20Not%20Valid
        (if (and (Utilities|Enum|Equal(Enum) (Variables|Flag|GetProgramState) "NewEnumerator5") (Variables|Flag|GetImageTrackingAccurateProgressFinished))
          (Variables|Default|SetTracked%20Geometry 0)
          (Default|HideProgressCanvas _fittoscanwidget_2)
          (Default|ResetProgressBar _fittoscanwidget_2))))
    (elif (Utilities|Enum|Equal(Enum) (Variables|Flag|GetProgramState) "NewEnumerator6")
      (Widget|RemovefromParent (Variables|UI|GetFitToScanWidget))
      (CallFunction|SpawnModel))))

(event Input|KeyboardEvents|AndroidBack
  (params (Key :type Key%20Structure :default "None"))
  ;[1 1 1] Android Back Button Pressed
  (:Pressed
    (if (Variables|Flag|GetQuitPromptIsShown?)
      (Game|QuitGame 0 "Quit" false)
      (else
        (CallFunction|ShowQuitPrompt)))))

(event Input|KeyboardEvents|AndroidMenu
  (params (Key :type Key%20Structure :default "None"))
  ;[1 1 1] Android Menu Pressed
  (:Pressed
    (Default|ToggleMainMenuShow (Variables|UI|GetMainMenuWidget))))

(fn ConstructionScript)

(fn ScanandDetectARImage
  (LocalVariables|SetTrackedGeometry_L 0)
  (bind _returnvalue (Class|ARBlueprintLibrary|GetAllGeometries))
  (bind _array_element (Utilities|Array|ForEachLoopwithBreak _returnvalue :!label _label)
    (:LoopBody
      (Utilities|Casting|CastToARTrackedImage _array_element)
      (LocalVariables|SetTrackedGeometry_L _array_element)
      (goto _label Break))
    (:Completed
      (return (LocalVariables|GetTrackedGeometry_L)))))